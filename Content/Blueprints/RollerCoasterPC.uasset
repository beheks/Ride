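; RollerCoasterPC is a VR player controller for a roller coaster, providing headset input and a gaze check for targets.
; Input actions reset HMD orientation and position or turn stereo on through a console command.
; CheckForInteractiveObjects sphere-traces along camera forward from an eye-height-raised start, with debug drawing.
; It stores the hit location and component, and returns the actor, component and whether the actor is tagged Target.
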(event `InputAction|ResetHMD`
  ;[1 1 1] Reset HMD
  (:`Released`
    (`HeadMountedDisplayFunctionLibrary.ResetOrientationAndPosition` 0.0)))

(event `InputAction|StereoOn`
  (:`Pressed`
    (`KismetSystemLibrary.ExecuteConsoleCommand` "stereo on")))

(fn `Check For Interactive Objects`
  (returns (HItTarget :type Boolean) (Component :type "PrimitiveComponent Object Reference") (Actor :type "Actor Object Reference"))
  (bind _playercameramanager (`self.PlayerCameraManager`))
  (bind _returnvalue (`self.K2_GetActorLocation` _playercameramanager))
  (bind _outhit (`KismetSystemLibrary.SphereTraceSingle_NEW` (`KismetMathLibrary.MakeVector` (.x _returnvalue) (.y _returnvalue) (+ (.z _returnvalue) (`Pawn.BaseEyeHeight` (`GameplayStatics.GetPlayerPawn` 0)))) (+ _returnvalue (* (`self.GetActorForwardVector` _playercameramanager) (`self.InteractionDistance`))) 1.0 "TraceTypeQuery2" false (`|MakeArray` (`GameplayStatics.GetPlayerPawn` 0) :!type "Actor Object Reference") "ForOneFrame"))
  (if true
    (bind (_location _normal _impactpoint _impactnormal _physmat _hitactor _hitcomponent) (`GameplayStatics.BreakHitResult` _outhit))
    (set `self.ImpactPoint` _location)
    (set `self.LookingAtComponent` _hitcomponent)
    (return (`self.ActorHasTag` _hitactor "Target") _hitcomponent _hitactor)))

(fn `UserConstructionScript`)