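; RideGameMode provides a check for what interactive object the player camera is looking at.
; CheckForInteractivity runs an object-type line trace along the camera's forward vector out to InteractionDistance, ignoring the player pawn.
; A hit stores the impact point and component, then returns the component, its actor and whether that component carries the "Interactive" tag.
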(fn `Check For Interactivity`
  (returns (`Hit Interactive Object` :type Boolean) (Component :type "PrimitiveComponent Object Reference") (Actor :type "Actor Object Reference"))
  (bind _returnvalue (`GameplayStatics.GetPlayerCameraManager` 0))
  (bind _returnvalue_2 (`self.K2_GetActorLocation` _returnvalue))
  (bind (_outhit _returnvalue_3) (`KismetSystemLibrary.LineTraceSingleForObjects` _returnvalue_2 (+ _returnvalue_2 (* (`self.GetActorForwardVector` _returnvalue) (`self.InteractionDistance`))) (`|MakeArray` "ObjectTypeQuery2" "ObjectTypeQuery1" "ObjectTypeQuery4" :!type "EngineTypes.EObjectTypeQuery Enum") false (`|MakeArray` (`GameplayStatics.GetPlayerPawn` 0) :!type "Actor Object Reference")))
  (if _returnvalue_3
    (bind (_location _normal _impactpoint _impactnormal _physmat _hitactor _hitcomponent) (`GameplayStatics.BreakHitResult` _outhit))
    (set `self.ImpactPoint` _impactpoint)
    (set `self.LookingAtComponent` _hitcomponent)
    (return (`ActorComponent.ComponentHasTag` _hitcomponent "Interactive") _hitcomponent _hitactor)))

(fn `UserConstructionScript`)