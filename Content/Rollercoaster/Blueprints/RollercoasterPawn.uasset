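; RollercoasterPawn is the rollercoaster ride pawn, and this Blueprint handles its ride audio.
; Climb and fall events crossfade between the GearsSound and TrackSound components, with gears heard on climbs and track noise on drops.
; Separate events fade the track sound out slowly or stop it with a quick fade.
; A helper function computes Euclidean distance between two vectors but is not called here.
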(event `FadeTrackSound`
  (`AudioComponent.FadeOut` (`self.TrackSound`) 3.0 0.0 :!label _label))

(event `StartClimbing`
  (`AudioComponent.FadeIn` (`self.GearsSound`) 6.0 1.0 0.0)
  (goto _label))

(event `StartFalling`
  (`AudioComponent.FadeIn` (`self.TrackSound`) 3.0 1.0 0.0)
  (`AudioComponent.FadeOut` (`self.GearsSound`) 1.0 0.0))

(event `StopTrackSound`
  (`AudioComponent.FadeOut` (`self.TrackSound`) 0.5 0.0))

(fn `Euclidian Distance`
  (params (`Vector 1` :type "Object.Vector Structure") (`Vector 2` :type "Object.Vector Structure"))
  (returns (Distance :type "Float (double-precision)"))
  (return (`KismetMathLibrary.Sqrt` (+ (`KismetMathLibrary.Square` (.x (- `Vector 1` `Vector 2`))) (`KismetMathLibrary.Square` (.y (- `Vector 1` `Vector 2`))) (`KismetMathLibrary.Square` (.z (- `Vector 1` `Vector 2`)))))))

(fn `UserConstructionScript`)