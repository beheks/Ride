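; Sphere projectile target that is destroyed after being looked at long enough, awarding a point to the Placar scoreboard.
; Construction creates a dynamic material with the color and transition parameters, and randomizes movement speed and upward-biased direction.
; UpdateMaterial accumulates gaze time directly in the material's SecondsLookedAt parameter, which doubles as the timer.
; At the transition length, it spawns particles, plays a random pitch-varied explosion sound, scores and destroys itself.
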(fn `Play Explosion Sound`
  (bind _explosion_sounds (`self.Explosion Sounds`))
  (`GameplayStatics.PlaySoundAtLocation` (`KismetArrayLibrary.Array_Get` _explosion_sounds (`KismetMathLibrary.RandomIntegerInRange` 0 (- (`KismetArrayLibrary.Array_Length` _explosion_sounds) 1))) (.location (`self.GetTransform` self)) 1.0 (`KismetMathLibrary.RandomFloatInRange` 0.8 1.2)))

(fn `Spawn Emitter`
  (`GameplayStatics.SpawnEmitterAtLocation` "/Game/Particles/BallDestroyed.BallDestroyed" (.location (`self.GetTransform`))))

(fn `Update Material`
  (params (`Delta Seconds` :type "Float (double-precision)") (Placar :type "Actor Object Reference (by ref)"))
  (bind _returnvalue (`MaterialInstanceDynamic.K2_GetScalarParameterValue` (`self.Sphere Material`) "SecondsLookedAt"))
  (if (>= _returnvalue (`self.TransistionLength`))
    (`self.Spawn Emitter`)
    (`self.Play Explosion Sound`)
    (bind _asplacar_c (cast `/Game/Blueprints/Placar` Placar))
    (`/Game/Blueprints/Placar.Update Score` _asplacar_c 1)
    (`self.K2_DestroyActor`)
    (else
      (`MaterialInstanceDynamic.SetScalarParameterValue` (`self.Sphere Material`) "SecondsLookedAt" (+ _returnvalue `Delta Seconds`)))))

(fn `UserConstructionScript`
  (bind _projectile_movement (`self.Projectile Movement`))
  (bind _sphere_material (`self.Sphere Material`))
  (bind _returnvalue (`PrimitiveComponent.CreateDynamicMaterialInstance` (`self.SM_Projectile`) 0 null))
  (set `self.Sphere Material` _returnvalue)
  (`MaterialInstanceDynamic.SetVectorParameterValue` _sphere_material "DiffuseColor" (`self.BaseColor`))
  (`MaterialInstanceDynamic.SetVectorParameterValue` _sphere_material "TimeColor" (`self.TimeBaseColor`))
  (`MaterialInstanceDynamic.SetScalarParameterValue` _sphere_material "TransitionLength" (`self.TransistionLength`))
  (set `ProjectileMovementComponent.InitialSpeed` (`KismetMathLibrary.RandomFloatInRange` (`self.Max Speed`) (`self.Min Speed`)) _projectile_movement)
  (set `MovementComponent.Velocity` (`KismetMathLibrary.MakeVector` (`KismetMathLibrary.RandomFloatInRange` -1.0 1.0) (`KismetMathLibrary.RandomFloatInRange` -1.0 1.0) (`KismetMathLibrary.RandomFloatInRange` 0.0 1.0)) _projectile_movement))